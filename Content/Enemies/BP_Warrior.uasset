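; BP_Warrior is an enemy that chases the player and shows a floating health bar.
; A Chase event runs AIMoveTo toward the player character from BeginPlay and calls itself only when a move succeeds, so a failed move ends the chase.
; BeginPlay caches the progress bar from BP_EnemyHPWidget.
; Each Tick updates it from the Health ratio and rotates the shadowless widget component to face the camera.
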(event `Chase`
  (`|AIMoveTo` self (0.0 0.0 0.0) (`GameplayStatics.GetPlayerCharacter` 0)
    (:`OnSuccess`
      (`self.Chase`))))

(event `self.ReceiveBeginPlay`
  (bind _asbp_enemy_hpwidget (cast `/Game/Enemies/BP_EnemyHPWidget` (`WidgetComponent.GetWidget` (`self.HPWidget`))))
  (set `self.HPProgress Bar` (`/Game/Enemies/BP_EnemyHPWidget.HPProgressBar` _asbp_enemy_hpwidget))
  (`self.Chase`))

(event `self.ReceiveTick`
  (params (DeltaSeconds :type "Float (single-precision)"))
  (bind _hpwidget (`self.HPWidget`))
  (bind _health (`self.Health`))
  (`ProgressBar.SetPercent` (`self.HPProgress Bar`) (/ (`HealthComponent.GetHealth` _health) (`HealthComponent.GetMaxHealth` _health)))
  (`SceneComponent.K2_SetWorldRotation` _hpwidget (`KismetMathLibrary.FindLookAtRotation` (`SceneComponent.K2_GetComponentLocation` _hpwidget) (`SceneComponent.K2_GetComponentLocation` (`PlayerCameraManager.TransformComponent` (`GameplayStatics.GetPlayerCameraManager` 0)))) false false))

(fn `UserConstructionScript`
  (`PrimitiveComponent.SetCastShadow` (`self.HPWidget`) false))