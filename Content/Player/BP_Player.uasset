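; Player character Blueprint with an HP bar widget, a hand-socketed sword, melee attacks and ragdoll death.
; Left click drives the Attack component, whose event locks movement into Custom mode while a slash montage plays.
; A montage notify sphere-traces forward for pawns, damages their HealthComponent and reports the hit to AI perception.
; Health's death event ragdolls the mesh, and F makes AI-audible noise with explosion effects.
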(event `self.ReceiveBeginPlay`
  ;[1 1 1] PlayerHPBar
  (bind _returnvalue (`|GenericCreateObject` "/Game/Player/BP_PlayerHPWidget.BP_PlayerHPWidget_C"))
  (bind _output_get (set `self.PlayerHPWidget` _returnvalue))
  (`UserWidget.AddToViewport` _output_get 0)
  ;[1 1 1] Sword
  (bind _returnvalue_2 (`|SpawnActorFromClass` "/Game/Weapons/BP_Sword.BP_Sword_C" (`self.GetTransform`) "Undefined" "OverrideRootScale" null null))
  (bind _output_get_2 (set `self.WeaponActor` _returnvalue_2))
  (`self.K2_AttachToComponent` _output_get_2 (`self.Mesh`) "hand_r_sword_socket" "SnapToTarget" "SnapToTarget" "SnapToTarget" true))

(event `Key|LeftMouseButton`
  (params (Key :type "Key Structure"))
  ;[1 1 1] OnAttack
  (:`Pressed`
    (`AttackComponent.CallAttack` (`self.Attack`))))

(event `self.Attack.OnAttack`
  (bind _returnvalue (`self.K2_GetActorLocation`))
  (bind _charactermovement (`self.CharacterMovement`))
  ;[1 1 1] OnAttack
  (switch `EMovementMode` (`CharacterMovementComponent.MovementMode` (`self.CharacterMovement`))
    (:`MOVE_None`
      _)
    (:`MOVE_Walking`
      _)
    (:`MOVE_NavWalking`
      _))
  (if (not (`self.IsAttacking`))
    (set `self.IsAttacking` true)
    (`CharacterMovementComponent.SetMovementMode` _charactermovement "MOVE_Custom" 0)
    (`MovementComponent.SetUpdatedComponent` _charactermovement (`self.Mesh`))
    (`self.AddControllerYawInput` 0.0)
    (bind _notifyname (`|PlayMontage` (`self.Mesh`) "/Game/Animations/sword-slash_Montage.sword-slash_Montage")
      (:`OnCompleted`
        (set `self.IsAttacking` false :!label _label)
        (`CharacterMovementComponent.SetMovementMode` (`self.CharacterMovement`) "MOVE_Walking" 0))
      (:`OnInterrupted`
        (goto _label))
      (:`OnNotifyBegin`
        (switch `name` _notifyname
          (:`SwordHit`
            (bind (_outhit _returnvalue_2) (`KismetSystemLibrary.SphereTraceSingleForObjects` :`Start` _returnvalue :`End` (+ _returnvalue (* (`self.GetActorForwardVector`) (100.0 100.0 100.0))) :`Radius` 20.0 :`ObjectTypes` (`|MakeArray` "ObjectTypeQuery3" :!type "EObjectTypeQuery Enum") :`DrawDebugType` "ForDuration" :`DrawTime` 1.0))
            (if _returnvalue_2
              (bind (_bblockinghit _binitialoverlap _time _distance _location _impactpoint _normal _impactnormal _physmat _hitactor) (`GameplayStatics.BreakHitResult` _outhit))
              (`HealthComponent.TakeDamage` (`self.GetComponentByClass` _hitactor "/Script/WarriorAIProject.HealthComponent") 200.0)
              (`AISense_Damage.ReportDamageEvent` _hitactor self 200.0 (`self.K2_GetActorLocation`)))))))))

(event `self.Health.OnDeath`
  (bind _mesh (`self.Mesh`))
  ;[1 1 1] Death
  (`PrimitiveComponent.SetSimulatePhysics` _mesh true)
  (`PrimitiveComponent.SetCollisionEnabled` _mesh "QueryAndPhysics")
  (`CharacterMovementComponent.DisableMovement` (`self.CharacterMovement`)))

(event `Key|F`
  (params (Key :type "Key Structure"))
  (bind _returnvalue (`self.K2_GetActorLocation`))
  ;[1 1 1] Make noise on F
  (:`Pressed`
    (`self.MakeNoise` 1.0 self _returnvalue)
    (`GameplayStatics.SpawnEmitterAtLocation` "/Game/StarterContent/Particles/P_Explosion.P_Explosion" _returnvalue)
    (`GameplayStatics.PlaySoundAtLocation` "/Game/StarterContent/Audio/Explosion_Cue.Explosion_Cue" _returnvalue (struct) 1.0 1.0 0.0 null null null null)))

(fn `UserConstructionScript`)